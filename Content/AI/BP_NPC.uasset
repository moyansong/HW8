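; BP_NPC is the NPC the player must protect, with an attribute component and a health bar widget.
; On BeginPlay it links itself to the health bar's WorldAttributeWidget and binds to health changes.
; When a health change leaves it dead, it shows a SettlementWidget with a Chinese failed-to-protect-NPC message.
; Each Tick scales the health bar inversely with distance to the player pawn, stretched wider horizontally.
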(event Custom|OnHealthChanged
  (params (InstigatocActor :type Actor%20Object%20Reference) (OwningCopmonent :type Attribute%20Component%20Object%20Reference) (NewHealth :type Float%20%28single-precision%29) (Damage :type Float%20%28single-precision%29))
  ;[1 1 1] The game ends when the NPC dies
  (if (not (Class|AttributeComponent|IsAlive (Variables|Default|GetAttributeComponent)))
    (bind _returnvalue (UserInterface|CreateWidget "/Game/ThirdPersonCPP/Blueprints/Widget/SettlementWidget.SettlementWidget_C"))
    (UserInterface|Viewport|AddtoViewport _returnvalue 0)
    (Rendering|Components|TextRender|SetText (Variables|/Game/ThirdPersonCPP/Blueprints/Widget/SettlementWidget.SettlementWidget_C|GetGameOverText _returnvalue) "守护NPC失败！！")))

(event EventBeginPlay
  (bind _asnpcattribute_widget (Utilities|Casting|CastToWorldAttributeWidget (UserInterface|GetWidget (Variables|Default|GetHealthBar))))
  (Variables|/Game/ThirdPersonCPP/Blueprints/Widget/WorldAttributeWidget.WorldAttributeWidget_C|SetNPC _asnpcattribute_widget self)
  (EventDispatchers|BindEventtoOnHealthChanged (Variables|Default|GetAttributeComponent) (delegate Custom|OnHealthChanged)))

(event Collision|EventActorBeginOverlap
  (params (OtherActor :type Actor%20Object%20Reference)))

(event EventTick
  (params (DeltaSeconds :type Float%20%28single-precision%29))
  ;[1 1 1] The health bar becomes smaller as the distance increases
  (CallFunction|SetHealthBarScale))

(fn ConstructionScript)

(fn SetHealthBarScale
  (bind _returnvalue (Game|Player|GetPlayerPawn 0))
  (bind _returnvalue_2 (Transformation|GetActorLocation))
  (bind _returnvalue_3 (Transformation|GetActorLocation _returnvalue))
  (bind _returnvalue_4 (- _returnvalue_2 _returnvalue_3))
  (bind _returnvalue_5 (Math|Vector|VectorLength _returnvalue_4))
  (bind _returnvalue_6 (/ 3e+02 _returnvalue_5))
  (Widget|Transform|SetRenderScale (UserInterface|GetWidget (Variables|Default|GetHealthBar)) (Math|Vector2D|MakeVector2D (* _returnvalue_6 3.0) _returnvalue_6)))